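; Actor component that makes its owning actor hover by bobbing it up and down along Z.
; BeginPlay randomizes amplitude and timescale per instance, with amplitude allowed to be negative, so hovering actors move differently.
; Each Tick adds a sine of game state time to the current height without sweeping, so the offset accumulates per frame and the travel depends on frame rate.
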(event EventBeginPlay
  (Variables|Default|SetHoverAmplitude (Math|Random|RandomFloatinRange -2.0 2.0))
  (Variables|Default|SetHoverTimescale (Math|Random|RandomFloatinRange 0.1 2.0)))

(event EventTick
  (params (DeltaSeconds :type Float%20%28single-precision%29))
  (bind _returnvalue (Components|GetOwner))
  (bind _returnvalue_2 (Transformation|GetActorLocation _returnvalue))
  (bind (_x _y _z) (Math|Vector|BreakVector _returnvalue_2))
  (Transformation|SetActorLocation _returnvalue (Math|Vector|MakeVector _x _y (+ _z (* (Math|Trig|Sin(Radians) (* (Actor|GetGameTimeSinceCreation (Game|GetGameState)) (Variables|Default|GetHoverTimescale))) (Variables|Default|GetHoverAmplitude)))) false false))