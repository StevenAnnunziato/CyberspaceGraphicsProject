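; Enemy actor that homes in on the player pawn and stops once it touches it.
; BeginPlay picks a random move speed, and each Tick steps the actor toward the player along the normalized direction and turns it to face them.
; Movement is a fixed per-frame offset without sweep or delta-time scaling.
; Overlapping the player sets a PlayerKilled flag, which halts the chase.
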(event EventBeginPlay
  (Variables|Default|SetMoveSpeed (Math|Random|RandomFloatinRange 1.5 3.0)))

(event Collision|EventActorBeginOverlap
  (params (OtherActor :type Actor%20Object%20Reference))
  (if (Collision|IsOverlappingActor (Game|Player|GetPlayerPawn 0) :!class /Script/Engine.Actor)
    (Variables|Default|SetPlayerKilled true)))

(event EventTick
  (params (DeltaSeconds :type Float%20%28single-precision%29))
  (if (not (Variables|Default|GetPlayerKilled))
    (Transformation|SetActorLocation (+ (Transformation|GetActorLocation) (* (Math|Vector|Normalize (- (Transformation|GetActorLocation (Game|Player|GetPlayerPawn 0)) (Transformation|GetActorLocation))) (Variables|Default|GetMoveSpeed))) false false)
    (Transformation|SetActorRotation (Math|Rotator|FindLookatRotation (Transformation|GetActorLocation) (Transformation|GetActorLocation (Game|Player|GetPlayerPawn 0))))))

(fn ConstructionScript)